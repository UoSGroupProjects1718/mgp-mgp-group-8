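; Conveyor belt actor for food that spawns a single sushi actor at its start location on BeginPlay.
; The construction script builds a spline between the start and end location components.
; A timeline meant to slide the food along that spline and destroy it at the end is unwired, as is the food assignment, so neither runs.
; A delayed for-loop macro is defined but unused.
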(event `self.ReceiveBeginPlay`
  (`self.Spawn`))

(event `Spawn`
  (bind _returnvalue (`|SpawnActorFromClass` "/Game/Blueprints/BP_Food_Sushi.BP_Food_Sushi_C" (`SceneComponent.K2_GetComponentToWorld` (`self.StartLocation`)) "Undefined" "OverrideRootScale" null null)))

(fn `UserConstructionScript`
  (bind _returnvalue (`AddComponent|NODE_AddSplineComponent-0`))
  (set `self.Spline` _returnvalue)
  (`SplineComponent.SetSplinePoints` (`self.Spline`) (`|MakeArray` (`SceneComponent.K2_GetComponentLocation` (`self.StartLocation`)) (`SceneComponent.K2_GetComponentLocation` (`self.EndLocation`))) "World" true))