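; BP_PlayerController is a player controller that adds rounds to two local players in alternation on touch input.
; Each touch press runs a FlipFlop that selects player controller 0 or 1, casts its PlayerState to BP_PlayerState and calls AddRound on it.
; The construction script only calls the parent version.
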(event `InputTouch`
  (params (Location :type "Vector Structure") (FingerIndex :type "ETouchIndex Enum"))
  (:`Pressed`
    (`/Engine/EditorBlueprintResources/StandardMacros.FlipFlop`
      (:`A`
        (bind _asbp_player_controller (cast `/Game/Blueprints/BP_PlayerController` (`GameplayStatics.GetPlayerController` 0)))
        (bind _asbp_player_state (cast `/Game/Blueprints/BP_PlayerState` (`Controller.PlayerState` _asbp_player_controller)))
        (`/Game/Blueprints/BP_PlayerState.AddRound` _asbp_player_state))
      (:`B`
        (bind _asbp_player_controller_2 (cast `/Game/Blueprints/BP_PlayerController` (`GameplayStatics.GetPlayerController` 1)))
        (bind _asbp_player_state_2 (cast `/Game/Blueprints/BP_PlayerState` (`Controller.PlayerState` _asbp_player_controller_2)))
        (`/Game/Blueprints/BP_PlayerState.AddRound` _asbp_player_state_2)))))

(fn `UserConstructionScript`
  (`parent.UserConstructionScript`))