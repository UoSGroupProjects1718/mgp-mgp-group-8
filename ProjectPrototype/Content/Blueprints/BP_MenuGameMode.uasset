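; BP_MenuGameMode is a game mode that brings up the menu UI when play begins.
; On BeginPlay it casts the first player controller to BP_MenuPlayerController, then creates MenuWidgetClass for it and adds it to the viewport.
; Input switches to UI-only with the widget focused and the mouse unlocked, followed by a debug print.
; A menu music node is present but unconnected, so it never plays.
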(event `self.ReceiveBeginPlay`
  (bind _asbp_menu_player_controller (cast `/Game/Blueprints/BP_MenuPlayerController` (`GameplayStatics.GetPlayerController` 0)))
  (bind _returnvalue (`|CreateWidget` (`self.MenuWidgetClass`) _asbp_menu_player_controller))
  (`UserWidget.AddToViewport` _returnvalue 0)
  (`WidgetBlueprintLibrary.SetInputMode_UIOnlyEx` _asbp_menu_player_controller _returnvalue)
  (`KismetSystemLibrary.PrintString` "Menu"))

(fn `UserConstructionScript`
  (`parent.UserConstructionScript`))