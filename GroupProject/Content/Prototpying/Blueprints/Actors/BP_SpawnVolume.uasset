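; BP_SpawnVolume is a prototype spawner actor that creates a new ShapeClass actor every second during play.
; A looping timer started on BeginPlay calls SpawnShape, which spawns at the actor's own location with default rotation and scale, adjusting for collisions but always spawning.
; EndPlay clears the stored timer handle.
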(event `self.ReceiveBeginPlay`
  (bind _returnvalue (`KismetSystemLibrary.K2_SetTimer` null "SpawnShape" 1.0 true))
  (set `self.TempHandle` _returnvalue))

(event `SpawnShape`
  (bind _returnvalue (`|SpawnActorFromClass` (`self.ShapeClass`) (`KismetMathLibrary.MakeTransform` (`self.K2_GetActorLocation`)) "AdjustIfPossibleButAlwaysSpawn" "OverrideRootScale" null null))
  (`/Engine/EditorBlueprintResources/StandardMacros.IsValid` _returnvalue))

(event `self.ReceiveEndPlay`
  (params (EndPlayReason :type "EEndPlayReason Enum" :default "Destroyed"))
  (`KismetSystemLibrary.K2_ClearAndInvalidateTimerHandle` (`self.TempHandle`)))

(fn `UserConstructionScript`)