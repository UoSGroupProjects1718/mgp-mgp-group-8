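; Experimental game state for a turn-based two-player match with debug-print feedback.
; A looping timer set to the round time flip-flops the controller ID between players, adding a turn to the new player's state.
; CheckRounds advances rounds when turn counts match, reading player indices 0 and 2 rather than 0 and 1.
; CheckWin compares scores at the round limit, favouring player one if lower; neither check is called here.
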(event `self.ReceiveBeginPlay`
  (`|ExecutionSequence`
    (:`then_0`
      (bind _returnvalue (`KismetSystemLibrary.K2_SetTimer` null "SwitchPlayer" (`self.RoundTime`) true))
      (set `self.TempHandle` _returnvalue))
    (:`then_1`
      (set `self.Rounds` (`self.Rounds`)))))

(event `SwitchPlayer`
  (`/Engine/EditorBlueprintResources/StandardMacros.FlipFlop`
    (:`A`
      (`GameplayStatics.SetPlayerControllerID` null 1)
      (`KismetSystemLibrary.PrintString` "PlayerTwo")
      (bind _asbp_player_state (cast `/Game/Experimental/BP_PlayerState` (`Controller.PlayerState` (`GameplayStatics.GetPlayerController` 1))))
      (`/Game/Experimental/BP_PlayerState.AddTurn` _asbp_player_state))
    (:`B`
      (`GameplayStatics.SetPlayerControllerID` null)
      (`KismetSystemLibrary.PrintString` "PlayerOne")
      (bind _asbp_player_state_2 (cast `/Game/Experimental/BP_PlayerState` (`Controller.PlayerState` (`GameplayStatics.GetPlayerController` 0))))
      (`/Game/Experimental/BP_PlayerState.AddTurn` _asbp_player_state_2))))

(event `CheckRounds`
  (`|ExecutionSequence`
    (:`then_0`
      (bind _asbp_player_state (cast `/Game/Experimental/BP_PlayerState` (`Controller.PlayerState` (`GameplayStatics.GetPlayerController` 0)))))
    (:`then_1`
      (bind _asbp_player_state_2 (cast `/Game/Experimental/BP_PlayerState` (`Controller.PlayerState` (`GameplayStatics.GetPlayerController` 2))))))
  (if (== (`/Game/Experimental/BP_PlayerState.Turns` _asbp_player_state) (`/Game/Experimental/BP_PlayerState.Turns` _asbp_player_state_2))
    (`self.IncreaseRounds`)))

(event `self.ReceiveEndPlay`
  (params (EndPlayReason :type "EEndPlayReason Enum" :default "Destroyed"))
  (`KismetSystemLibrary.K2_ClearAndInvalidateTimerHandle` (`self.TempHandle`)))

(fn `CheckScore`
  (`|ExecutionSequence`
    (:`then_0`
      (bind _asbp_player_controller (cast `/Game/Experimental/BP_PlayerController` (`GameplayStatics.GetPlayerController` 0)))
      (bind _asbp_player_state (cast `/Game/Experimental/BP_PlayerState` (`Controller.PlayerState` _asbp_player_controller))))
    (:`then_1`
      (bind _asbp_player_controller_2 (cast `/Game/Experimental/BP_PlayerController` (`GameplayStatics.GetPlayerController` 1)))
      (bind _asbp_player_state_2 (cast `/Game/Experimental/BP_PlayerState` (`Controller.PlayerState` _asbp_player_controller_2)))))
  (if (< (`/Game/Experimental/BP_PlayerState.GetScore` _asbp_player_state) (`/Game/Experimental/BP_PlayerState.GetScore` _asbp_player_state_2))
    (`KismetSystemLibrary.PrintString` "Player One Wins!")
    (else
      (`KismetSystemLibrary.PrintString` "Player Two Wins!"))))

(fn `CheckWin`
  (if (== (`self.MaxRounds`) (`self.Rounds`))
    (`self.CheckScore`)
    (`KismetSystemLibrary.PrintString` "Notify winning player")))

(fn `IncreaseRounds`
  (if (< (`self.Rounds`) (`self.MaxRounds`))
    (bind _output_get (set `self.Rounds` (+ (`self.Rounds`) 1)))
    (`KismetSystemLibrary.PrintString` (`KismetStringLibrary.Conv_IntToString` _output_get))))

(fn `UserConstructionScript`
  (`parent.UserConstructionScript`))