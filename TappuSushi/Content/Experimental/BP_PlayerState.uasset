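; BP_PlayerState is a player state Blueprint that tracks a player's score and turn count.
; BeginPlay sets the turn count to its maximum.
; AddScore accumulates points into the score, and GetScore returns it.
; Despite its name, AddTurn decrements the count when it is at or below the maximum and prints the result, with no lower bound.
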(event `self.ReceiveBeginPlay`
  (set `self.Turns` (`self.MaxTurns`)))

(fn `AddScore`
  (params (Score :type Integer))
  (set `self.PlayerScore` (+ Score (`self.PlayerScore`))))

(fn `AddTurn`
  (if (<= (`self.Turns`) (`self.MaxTurns`))
    (bind _output_get (set `self.Turns` (- (`self.Turns`) 1)))
    (`KismetSystemLibrary.PrintString` (`KismetStringLibrary.Conv_IntToString` _output_get))))

(fn `GetScore`
  (returns (NewParam :type Integer))
  (return (`self.PlayerScore`)))

(fn `UserConstructionScript`)